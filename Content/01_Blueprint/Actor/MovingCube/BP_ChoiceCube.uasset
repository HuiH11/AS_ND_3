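; BP_ChoiceCube is a moving cube that shuttles its StaticMesh back and forth between its starting relative location and the TargetComp location.
; Each Tick it measures distance travelled against the path length, swaps start and target on arrival, and moves the mesh at a constant Speed.
; The IsWaitCube flag chooses between pausing for a fixed few seconds at each end and moving continuously.
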(event `self.ReceiveBeginPlay`
  (set `self.StartLocation` (`SceneComponent.RelativeLocation` (`self.StaticMesh`)))
  (set `self.TargetLocation` (`SceneComponent.RelativeLocation` (`self.TargetComp`))))

(event `self.ReceiveTick`
  (params (DeltaSeconds :type "Float (single-precision)"))
  (if (`self.Is Wait Cube`)
    (`self.WaitMove` DeltaSeconds)
    (else
      (`self.DontStopMove` DeltaSeconds))))

(fn `DontStopMove`
  (params (DeltaTime :type "Float (double-precision)"))
  (`self.LenthCheck`)
  (`self.Shuffle`)
  (`self.MoveUpdate` DeltaTime))

(fn `LenthCheck`
  ;[1 1 1] 가야할 거리
  (set `self.Length` (`KismetMathLibrary.VSize` (- (`self.TargetLocation`) (`self.StartLocation`))))
  ;[1 1 1] 온 거리
  (set `self.Travelled` (`KismetMathLibrary.VSize` (- (`SceneComponent.RelativeLocation` (`self.StaticMesh`)) (`self.StartLocation`)))))

(fn `MoveUpdate`
  (params (DeltaTime :type "Float (double-precision)"))
  ;[1 1 1] 이동
  (`SceneComponent.K2_SetRelativeLocation` (`self.StaticMesh`) (+ (* (* DeltaTime (`self.Speed`)) (`KismetMathLibrary.Normal` (- (`self.TargetLocation`) (`self.StartLocation`)))) (`SceneComponent.RelativeLocation` (`self.StaticMesh`))) false false))

(fn `Shuffle`
  (returns (IsChange :type Boolean))
  ;[1 1 1] 위치 셔플
  (if (>= (`self.Travelled`) (`self.Length`))
    (set `self.TempLocation` (`self.StartLocation`))
    (set `self.StartLocation` (`self.TargetLocation`))
    (set `self.TargetLocation` (`self.TempLocation`))
    (return true)
    (else
      (return false))))

(fn `UserConstructionScript`)

(fn `WaitMove`
  (params (DeltaTime :type "Float (double-precision)"))
  (if (`self.IsWait`)
    (`self.WaitTimeCheck` DeltaTime)
    (else
      (`self.LenthCheck`)
      (bind _ischange (`self.Shuffle`))
      (set `self.IsWait` _ischange)
      (`self.MoveUpdate` DeltaTime))))

(fn `WaitTimeCheck`
  (params (DeltaTime :type "Float (double-precision)"))
  (bind _output_get (set `self.AccTime` (+ DeltaTime (`self.AccTime`))))
  (if (>= _output_get 3.0)
    (set `self.IsWait` false)
    (set `self.AccTime` 0.0)))