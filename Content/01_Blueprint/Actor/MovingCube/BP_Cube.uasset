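; BP_Cube is an actor that moves up and down continuously along the world Z axis at a constant speed set in BeginPlay.
; Each Tick accumulates elapsed time, picks an up or down direction from the Go flag, and offsets the location by direction, speed and delta time without sweeping.
; When the timer passes a fixed threshold of a few seconds, Go flips and the timer resets, reversing the motion.
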(event `self.ReceiveBeginPlay`
  ;[1 1 1] speed 초기화
  (set `self.Speed` 200.0))

(event `self.ReceiveTick`
  (params (DeltaSeconds :type "Float (single-precision)"))
  (`|ExecutionSequence`
    (:`then_0`
      ;[1 1 1] 시간 더하기
      (set `self.AccTime` (+ DeltaSeconds (`self.AccTime`))))
    (:`then_1`
      ;[1 1 1] go 값에 따른 dir 벡터 값 변경
      (if (`self.Go`)
        (set `self.Dir` (0.0 0.0 1.0))
        (else
          (set `self.Dir` (0.0 0.0 -1.0))))
      (`self.K2_SetActorLocation` (+ (`self.K2_GetActorLocation`) (* (`GameplayStatics.GetWorldDeltaSeconds`) (* (`KismetMathLibrary.Normal` (`self.Dir`)) (`self.Speed`))))))
    (:`then_2`
      ;[1 1 1] go 값 세팅
      (if (> (`self.AccTime`) 3.0)
        (if (`self.Go`)
          (set `self.Go` false)
          (else
            (set `self.Go` true)))
        (set `self.AccTime` 0.0)))))

(fn `UserConstructionScript`)