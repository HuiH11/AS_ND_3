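; BP_Floor is an interactive floor that disappears after a character steps on it and spawns a replacement of itself.
; A box overlap with BP_Base_Character sets a flag that makes Tick accumulate delta time until DestroyTime, then destroy the actor and clear ExistFloor.
; The second Tick sequence branch spawns a new BP_Floor whenever ExistFloor is false, using the transform saved at BeginPlay offset by MVector.
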(event `self.ReceiveBeginPlay`
  (set `self.ActorLocation` (`SceneComponent.K2_GetComponentToWorld` (`self.DefaultSceneRoot`))))

(event `self.ReceiveTick`
  (params (DeltaSeconds :type "Float (single-precision)"))
  (bind (_actorlocation_location _actorlocation_rotation _actorlocation_scale) (`KismetMathLibrary.BreakTransform` (`self.ActorLocation`)))
  (`|ExecutionSequence`
    (:`then_0`
      (if (`self.bPlayerOverlap`)
        (`self.Destroy`)))
    (:`then_1`
      (if (not (`self.bExistFloor`))
        (`|SpawnActorFromClass` "BP_Floor_C" (`KismetMathLibrary.MakeTransform` (+ (`self.MVector`) _actorlocation_location) _actorlocation_rotation _actorlocation_scale) "Undefined" "MultiplyWithRoot" null null)))))

(event `self.Box.OnComponentBeginOverlap`
  (params (OverlappedComponent :type "PrimitiveComponent Object Reference") (OtherActor :type "Actor Object Reference") (OtherComp :type "PrimitiveComponent Object Reference") (OtherBodyIndex :type Integer) (bFromSweep :type Boolean) (SweepResult :type "HitResult Structure (by ref)"))
  (bind _asbp_base_character (cast `/Game/01_Blueprint/Actor/Character/BP_Base_Character` OtherActor))
  (`/Engine/EditorBlueprintResources/StandardMacros.IsValid` _asbp_base_character
    (:`Is Valid`
      (set `self.bPlayerOverlap` true))))

(event `self.ReceiveDestroyed`)

(fn `Destroy`
  (set `self.AccTime` (+ (`GameplayStatics.GetWorldDeltaSeconds`) (`self.AccTime`)))
  (if (>= (`self.AccTime`) (`self.DestroyTime`))
    (`self.K2_DestroyActor`)
    (set `self.bExistFloor` false)))

(fn `Generate`)

(fn `UserConstructionScript`)