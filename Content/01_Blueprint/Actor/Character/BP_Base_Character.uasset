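; Base player character with Enhanced Input movement, camera zoom, spotlight toggle, dance and swappable weapon meshes.
; Attacks spend mana on a four-montage combo, with clicks buffered until ComboAction.
; AttackCheck sphere-traces hits, spawns effects and random damage numbers, and adds Android points shown on HUD and character widget.
; Also handles physical-material footsteps, Tick-driven dissolve, NPC interaction actors and hard-keyed mana refill, interaction and radial DiggingMessage.
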(event `self.ReceiveBeginPlay`
  (`|ExecutionSequence`
    (:`then_0`
      ;[1 1 1] 맵핑
      (bind `_as플레이어_컨트롤러` (cast `PlayerController` (`self.GetController`)))
      (`/Engine/EditorBlueprintResources/StandardMacros.IsValid` `_as플레이어_컨트롤러`
        (:`Is Valid`
          (`EnhancedInputSubsystemInterface.AddMappingContext` (pcsubsystem `EnhancedInputLocalPlayerSubsystem` `_as플레이어_컨트롤러`) "/Game/01_Blueprint/Global/Input/IM_Context.IM_Context" 0 (struct))
          (`PrimitiveComponent.CreateDynamicMaterialInstance` (`self.Mesh`) 0 "/Game/02_Resource/Character/Skeleton/skeleton_Inst.skeleton_Inst" "None"))))
    (:`then_1`
      (`self.ManaUpdate`))))

(event `EnhancedInput|/Game/01_Blueprint/Global/Input/IA_Jump`
  (params (ActionValue :type Boolean) (ElapsedSeconds :type "Float (double-precision)") (TriggeredSeconds :type "Float (double-precision)") (InputAction :type "InputAction Object Reference" :default "/Game/01_Blueprint/Global/Input/IA_Jump.IA_Jump"))
  ;[1 1 1] 점프
  (:`Started`
    (`self.Jump`)))

(event `EnhancedInput|/Game/01_Blueprint/Global/Input/IA_MoveFoward`
  (params (ActionValue :type "Float (double-precision)") (ElapsedSeconds :type "Float (double-precision)") (TriggeredSeconds :type "Float (double-precision)") (InputAction :type "InputAction Object Reference" :default "/Game/01_Blueprint/Global/Input/IA_MoveFoward.IA_MoveFoward"))
  (bind (_returnvalue_roll _returnvalue_pitch _returnvalue_yaw) (`KismetMathLibrary.BreakRotator` (`self.GetControlRotation`)))
  ;[1 1 1] 앞으로
  (:`Triggered`
    (`self.AddMovementInput` (`KismetMathLibrary.GetForwardVector` (`KismetMathLibrary.MakeRotator` 0.0 0.0 _returnvalue_yaw)) ActionValue)
    (set `self.IsMove` true :!label _label))
  (:`Completed`
    (set `self.IsMove` false :!label _label_2)))

(event `Key|H`
  (params (Key :type "Key Structure"))
  ;[1 1 1] 디졸브
  (:`Pressed`
    (set `self.DissolveOn` (not (`self.DissolveOn`)))))

(event `self.ReceiveTick`
  (params (DeltaSeconds :type "Float (single-precision)"))
  (`|ExecutionSequence`
    (:`then_0`
      ;[1 1 1] 디졸브
      (`self.Dissolve` DeltaSeconds DeltaSeconds))))

(event `EnhancedInput|/Game/01_Blueprint/Global/Input/IA_MoveRight`
  (params (ActionValue :type "Float (double-precision)") (ElapsedSeconds :type "Float (double-precision)") (TriggeredSeconds :type "Float (double-precision)") (InputAction :type "InputAction Object Reference" :default "/Game/01_Blueprint/Global/Input/IA_MoveRight.IA_MoveRight"))
  (bind (_returnvalue_roll _returnvalue_pitch _returnvalue_yaw) (`KismetMathLibrary.BreakRotator` (`self.GetControlRotation`)))
  ;[1 1 1] 옆으로
  (:`Triggered`
    (`self.AddMovementInput` (`KismetMathLibrary.GetRightVector` (`KismetMathLibrary.MakeRotator` 0.0 0.0 _returnvalue_yaw)) ActionValue)
    (goto _label))
  (:`Completed`
    (goto _label_2)))

(event `EnhancedInput|/Game/01_Blueprint/Global/Input/IA_Light`
  (params (ActionValue :type Boolean) (ElapsedSeconds :type "Float (double-precision)") (TriggeredSeconds :type "Float (double-precision)") (InputAction :type "InputAction Object Reference" :default "/Game/01_Blueprint/Global/Input/IA_Light.IA_Light"))
  ;[1 1 1] 라이트
  (:`Started`
    (if (`self.IsLight`)
      (`LightComponent.SetIntensity` (`self.SpotLight`) 0.0)
      (set `self.IsLight` false)
      (else
        (`LightComponent.SetIntensity` (`self.SpotLight`) 10000.0)
        (set `self.IsLight` true)))))

(event `EnhancedInput|/Game/01_Blueprint/Global/Input/IA_MouseXY`
  (params (ActionValue :type "Vector2D Structure") (ElapsedSeconds :type "Float (double-precision)") (TriggeredSeconds :type "Float (double-precision)") (InputAction :type "InputAction Object Reference" :default "/Game/01_Blueprint/Global/Input/IA_MouseXY.IA_MouseXY"))
  ;[1 1 1] 마우스 회전
  (:`Triggered`
    (`self.AddControllerYawInput` ActionValue_X)
    (`self.AddControllerPitchInput` ActionValue_Y)))

(event `EnhancedInput|/Game/01_Blueprint/Global/Input/IA_Dance`
  (params (ActionValue :type Boolean) (ElapsedSeconds :type "Float (double-precision)") (TriggeredSeconds :type "Float (double-precision)") (InputAction :type "InputAction Object Reference" :default "/Game/01_Blueprint/Global/Input/IA_Dance.IA_Dance"))
  ;[1 1 1] 춤
  (:`Triggered`
    (`|PlayMontage` (`self.Mesh`) "/Game/02_Resource/Character/Skeleton/MixamoAni/Sk_Dance.Sk_Dance"
      (:`then`
        (set `self.IsDance` false)))))

(event `EnhancedInput|/Game/01_Blueprint/Global/Input/IA_MouseWheel`
  (params (ActionValue :type "Float (double-precision)") (ElapsedSeconds :type "Float (double-precision)") (TriggeredSeconds :type "Float (double-precision)") (InputAction :type "InputAction Object Reference" :default "/Game/01_Blueprint/Global/Input/IA_MouseWheel.IA_MouseWheel"))
  (bind _springarm (`self.SpringArm`))
  ;[1 1 1] 확대 축소
  (:`Triggered`
    (set `SpringArmComponent.TargetArmLength` (`KismetMathLibrary.FClamp` (+ (* ActionValue 10.0) (`SpringArmComponent.TargetArmLength` _springarm)) 100.0 1100.0) _springarm)))

(event `AttackCheck`
  (bind _returnvalue (`KismetMathLibrary.RandomIntegerInRange` 1 100))
  (bind _returnvalue_2 (`SceneComponent.K2_GetComponentLocation` (`self.Weapon`)))
  ;[1 1 1] 공격 판정
  (bind (_outhit _returnvalue_3) (`KismetSystemLibrary.SphereTraceSingleByProfile` :`Start` _returnvalue_2 :`End` (+ _returnvalue_2 (* (`self.GetActorForwardVector`) 50.0)) :`Radius` 50.0 :`ProfileName` "PlayerAttack" :`DrawDebugType` "ForDuration"))
  (if _returnvalue_3
    (bind (_bblockinghit _binitialoverlap _time _distance _location _impactpoint) (`GameplayStatics.BreakHitResult` _outhit))
    (bind _returnvalue_4 (`NiagaraFunctionLibrary.SpawnSystemAtLocation` "/Game/02_Resource/Niagara/NA_AttackEffect.NA_AttackEffect" _location))
    (`NiagaraComponent.SetNiagaraVariableFloat` _returnvalue_4 "MaxSize" 20.0)
    (`self.AddAndroidP`)
    ;[1 1 1] 데미지 띄우기
    (bind _returnvalue_5 (`|SpawnActorFromClass` "/Game/01_Blueprint/UI/DMG_Actor.DMG_Actor_C" (`KismetMathLibrary.Conv_VectorToTransform` _impactpoint) "AlwaysSpawn" "MultiplyWithRoot" null null))
    (`/Game/01_Blueprint/UI/DMG_Actor.Init_DMGActor` _returnvalue_5 _returnvalue (> _returnvalue 70))))

(event `EnhancedInput|/Game/01_Blueprint/Global/Input/IA_MouseLeftClick`
  (params (ActionValue :type Boolean) (ElapsedSeconds :type "Float (double-precision)") (TriggeredSeconds :type "Float (double-precision)") (InputAction :type "InputAction Object Reference" :default "/Game/01_Blueprint/Global/Input/IA_MouseLeftClick.IA_MouseLeftClick"))
  ;[1 1 1] 공격(마우스 우클릭)
  (:`Started`
    (if (`self.IsAttack`)
      (set `self.AttackSave` true)
      (else
        (bind _attackable (`self.AttackSpentMana` :!label _label_3))
        (if _attackable
          (switch `int` (`self.ComboCount`)
            (:`0`
              (`|PlayMontage` (`self.Mesh`) "/Game/02_Resource/Character/Skeleton/BlendAnimation/AMT/AMT_Attack_Chop.AMT_Attack_Chop"
                (:`then`
                  (set `self.IsAttack` true)
                  (set `self.ComboCount` 1))))
            (:`1`
              (`|PlayMontage` (`self.Mesh`) "/Game/02_Resource/Character/Skeleton/BlendAnimation/AMT/AMT_Attack_Slice.AMT_Attack_Slice"
                (:`then`
                  (set `self.IsAttack` true)
                  (set `self.ComboCount` 2))))
            (:`2`
              (`|PlayMontage` (`self.Mesh`) "/Game/02_Resource/Character/Skeleton/BlendAnimation/AMT/AMT_Attack_Spin.AMT_Attack_Spin"
                (:`then`
                  (set `self.IsAttack` true)
                  (set `self.ComboCount` 3))))
            (:`3`
              (`|PlayMontage` (`self.Mesh`) "/Game/02_Resource/Character/Skeleton/BlendAnimation/AMT/AMT_Shoot.AMT_Shoot"
                (:`then`
                  (set `self.IsAttack` true)
                  (set `self.ComboCount` 0)))))
          (else
            (`self.ResetCombo`)
            (`KismetSystemLibrary.PrintString` "NO MANA!")))))))

(event `ComboAction`
  ;[1 1 1] 공격(마우스 우클릭)
  (if (`self.AttackSave`)
    (set `self.AttackSave` false)
    (goto _label_3)))

(event `Key|NumPadThree`
  (params (Key :type "Key Structure"))
  (bind _returnvalue (`self.K2_GetActorLocation`))
  (:`Pressed`
    (bind _outhits (`KismetSystemLibrary.SphereTraceMultiByProfile` :`Start` _returnvalue :`End` _returnvalue :`Radius` 500.0 :`ProfileName` "BlockAll" :`DrawDebugType` "ForDuration" :`DrawTime` 3.0))
    (for _array_element _outhits
      (message `/Game/01_Blueprint/Actor/Monster/Minion_Interface.Digging` (`.HitActor` (`GameplayStatics.BreakHitResult` _array_element)) "NewEnumerator0"))))

(event `ResetCombo`
  ;[1 1 1] 공격(마우스 우클릭)
  (set `self.AttackSave` false)
  (set `self.ComboCount` 0)
  (set `self.IsAttack` false))

(event `FootStep`
  (params (IsLeft :type Boolean))
  (`self.Func_FootStep` IsLeft))

(event `InteractionUIOn`
  (params (NPCLocation :type "Vector Structure"))
  (bind _returnvalue (`|SpawnActorFromClass` "/Game/01_Blueprint/UI/InteractionActor.InteractionActor_C" (`KismetMathLibrary.Conv_VectorToTransform` NPCLocation) "AlwaysSpawn" "MultiplyWithRoot" null null))
  (set `self.InteractionActor` _returnvalue))

(event `ManaUpdate`
  (bind _ascharacter_widget (cast `/Game/01_Blueprint/UI/CharacterWidget` (`WidgetComponent.GetWidget` (`self.Widget`))))
  (`/Game/01_Blueprint/UI/CharacterWidget.SetMPPercent` _ascharacter_widget (/ (`self.CurMana`) (`self.MaxMana`))))

(event `InteractionUIOff`
  (bind _interactionactor (`self.InteractionActor`))
  (`/Engine/EditorBlueprintResources/StandardMacros.IsValid` _interactionactor
    (:`Is Valid`
      (`KismetSystemLibrary.PrintString` "dd")
      (`self.K2_DestroyActor` _interactionactor)
      (set `self.InteractionActor` null))))

(event `Key|One`
  (params (Key :type "Key Structure"))
  (:`Pressed`
    (set `self.CurMana` (`self.MaxMana`))
    (`self.ManaUpdate`)))

(event `Key|Two`
  (params (Key :type "Key Structure"))
  (bind _interactionactor (`self.InteractionActor`))
  (:`Pressed`
    (set `/Game/01_Blueprint/UI/InteractionActor.ONInteraction` true _interactionactor)
    (`KismetSystemLibrary.PrintString` "on"))
  (:`Released`
    (set `/Game/01_Blueprint/UI/InteractionActor.ONInteraction` false _interactionactor)
    (`KismetSystemLibrary.PrintString` "off")))

(event `SetCharacterName`
  (bind _characterinfo_cname (break `/Game/01_Blueprint/Global/Structs/Character_Struct` (`self.CharacterInfo`)))
  (bind _ascharacter_widget (cast `/Game/01_Blueprint/UI/CharacterWidget` (`WidgetComponent.GetWidget` (`self.Widget`))))
  (`/Game/01_Blueprint/UI/CharacterWidget.SetName` _ascharacter_widget (`KismetTextLibrary.Conv_NameToText` _characterinfo_cname)))

(event `SetWeapon`
  (switch `int` (`self.WeaponNum`)
    (:`0`
      (`StaticMeshComponent.SetStaticMesh` (`self.Weapon`) "/Game/02_Resource/Character/Skeleton/Skeleton_Axe.Skeleton_Axe"))
    (:`1`
      (`StaticMeshComponent.SetStaticMesh` (`self.Weapon`) "/Game/02_Resource/Character/Skeleton/Skeleton_Blade.Skeleton_Blade"))
    (:`2`
      (`StaticMeshComponent.SetStaticMesh` (`self.Weapon`) "/Game/02_Resource/Character/Skeleton/Skeleton_Crossbow.Skeleton_Crossbow"))
    (:`3`
      (`StaticMeshComponent.SetStaticMesh` (`self.Weapon`) "/Game/02_Resource/Character/Skeleton/Skeleton_Staff.Skeleton_Staff"))))

(fn `AddAndroidP`
  (bind _result (`/Engine/EditorBlueprintResources/StandardMacros.IncrementInt` (`self.CurAndroidP`))
    (:`  `
      (if (> _result (`self.MaxAndroidP`))
        (set `self.CurAndroidP` (`self.MaxAndroidP`)))
      (if (== (`self.CurAndroidP`) (`self.MaxAndroidP`))
        (set `self.CompleteAnd` (+ (`self.CompleteAnd`) 1))
        (set `self.CurAndroidP` 0))
      (bind _asbp_main_hud (cast `/Game/01_Blueprint/FrameWork/BP_MainHUD` (`PlayerController.GetHUD` (`GameplayStatics.GetPlayerController` 0))))
      (`/Game/01_Blueprint/UI/MainUI.SetAndroidPPercent` (`/Game/01_Blueprint/FrameWork/BP_MainHUD.MainUI` _asbp_main_hud) (/ (`KismetMathLibrary.Conv_IntToDouble` (`self.CurAndroidP`)) (`KismetMathLibrary.Conv_IntToDouble` (`self.MaxAndroidP`))))
      (bind _ascharacter_widget (cast `/Game/01_Blueprint/UI/CharacterWidget` (`WidgetComponent.GetWidget` (`self.Widget`))))
      (`/Game/01_Blueprint/UI/CharacterWidget.SetAndroidPoint` _ascharacter_widget (`self.CompleteAnd`) (`self.MaxAnd`)))))

(fn `AttackSpentMana`
  (returns (AttackAble :type Boolean))
  (bind _returnvalue (- (`self.CurMana`) (`self.SpentMana`)))
  (bind _returnvalue_2 (>= _returnvalue 0.0))
  (if _returnvalue_2
    (set `self.CurMana` _returnvalue))
  (`self.ManaUpdate`)
  (return _returnvalue_2))

(fn `Dissolve`
  (params (B :type "Float (double-precision)") (B2 :type "Float (double-precision)"))
  (bind _dissolvetime (`self.Dissolvetime`))
  (bind _dissolvetime_2 (`self.Dissolvetime`))
  (bind _dissolvetime_3 (`self.Dissolvetime`))
  (if (`self.DissolveOn`)
    (if (> _dissolvetime -1.0)
      (bind _output_get (set `self.Dissolvetime` (- _dissolvetime B2)))
      (`MeshComponent.SetScalarParameterValueOnMaterials` (`self.Mesh`) "Dissolve" _output_get)
      (`MeshComponent.SetScalarParameterValueOnMaterials` (`self.Weapon`) "Dissolve" _dissolvetime_3))
    (elif (< _dissolvetime_2 2.0)
      (bind _output_get_2 (set `self.Dissolvetime` (+ _dissolvetime_2 B)))
      (`MeshComponent.SetScalarParameterValueOnMaterials` (`self.Mesh`) "Dissolve" _output_get_2)
      (`MeshComponent.SetScalarParameterValueOnMaterials` (`self.Weapon`) "Dissolve" _dissolvetime_3))))

(fn `Func_FootStep`
  (params (IsLeft :type Boolean))
  (bind _footlocation (`self.FootLocation`))
  (bind _returnvalue (`SceneComponent.K2_GetComponentRotation` (`self.Mesh`)))
  (if IsLeft
    (set `self.FootLocation` (`SceneComponent.GetSocketLocation` (`self.Mesh`) "toes_l"))
    (else
      (set `self.FootLocation` (`SceneComponent.GetSocketLocation` (`self.Mesh`) "toes_r"))))
  (bind (_outhit _returnvalue_2) (`KismetSystemLibrary.LineTraceSingle` :`Start` _footlocation :`End` (+ _footlocation (0.0 0.0 -20.0)) :`TraceChannel` "TraceTypeQuery3" :`DrawDebugType` "ForDuration" :`DrawTime` 2.0))
  (if _returnvalue_2
    (bind (_bblockinghit _binitialoverlap _time _distance _location _impactpoint _normal _impactnormal _physmat) (`GameplayStatics.BreakHitResult` _outhit))
    (bind _aspm_nd (cast `/Game/02_Resource/MTRL/PM_ND` _physmat))
    (`NiagaraFunctionLibrary.SpawnSystemAtLocation` (`/Game/02_Resource/MTRL/PM_ND.NaFootWalk` _aspm_nd) _impactpoint _returnvalue)
    (`GameplayStatics.PlaySoundAtLocation` (`/Game/02_Resource/MTRL/PM_ND.FootSound` _aspm_nd) _impactpoint (struct) 1.0 1.0 0.0 null null null null)
    (`|SpawnActorFromClass` (`/Game/02_Resource/MTRL/PM_ND.FootPrint` _aspm_nd) (`KismetMathLibrary.MakeTransform` _impactpoint (`KismetMathLibrary.ComposeRotators` _returnvalue (struct :`Yaw` 90.0))) "Undefined" "MultiplyWithRoot" null null)
    (else
      (`KismetSystemLibrary.PrintString` "NO"))))

(fn `Shooting`
  (bind (_returnvalue_location _returnvalue_rotation) (`KismetMathLibrary.BreakTransform` (`self.GetTransform`)))
  (`|SpawnActorFromClass` "/Game/01_Blueprint/Actor/Character/BP_ShootingBall.BP_ShootingBall_C" (`KismetMathLibrary.MakeTransform` (+ (* (`self.GetActorForwardVector`) 200.0) _returnvalue_location) _returnvalue_rotation) "Undefined" "MultiplyWithRoot" null null)
  (`NiagaraFunctionLibrary.SpawnSystemAtLocation` "/Game/02_Resource/Niagara/NA_FireEffect.NA_FireEffect" (+ (`SceneComponent.K2_GetComponentLocation` (`self.Weapon`)) (* (`self.GetActorForwardVector`) 50.0))))

(fn `UserConstructionScript`
  (`KismetArrayLibrary.Array_Add` (`SceneCaptureComponent.ShowOnlyActors` (`self.FaceSceneCapture`)) self))