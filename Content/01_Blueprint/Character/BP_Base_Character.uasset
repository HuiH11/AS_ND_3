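; Playable skeleton character with an axe, using Enhanced Input for movement, camera zoom, jumping, dancing and a spotlight toggle.
; Left-click plays a four-step montage combo, buffering presses until ComboAction, while AttackCheck sphere-traces from the axe for hit effects.
; H toggles a Tick-driven material dissolve on body and axe.
; Shooting spawns projectiles, and FootStep traces below each foot for physical-material-specific effects, sounds and footprints.
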(event `self.ReceiveBeginPlay`
  ;[1 1 1] 맵핑
  (bind `_as플레이어_컨트롤러` (cast `PlayerController` (`self.GetController`)))
  (`/Engine/EditorBlueprintResources/StandardMacros.IsValid` `_as플레이어_컨트롤러`
    (:`Is Valid`
      (`EnhancedInputSubsystemInterface.AddMappingContext` (pcsubsystem `EnhancedInputLocalPlayerSubsystem` `_as플레이어_컨트롤러`) "/Game/01_Blueprint/Global/Input/IM_Context.IM_Context" 0 (struct))
      (`PrimitiveComponent.CreateDynamicMaterialInstance` (`self.Mesh`) 0 "/Game/02_Resource/Character/Skeleton/skeleton_Inst.skeleton_Inst" "None"))))

(event `EnhancedInput|/Game/01_Blueprint/Global/Input/IA_Jump`
  (params (ActionValue :type Boolean) (ElapsedSeconds :type "Float (double-precision)") (TriggeredSeconds :type "Float (double-precision)") (InputAction :type "InputAction Object Reference" :default "/Game/01_Blueprint/Global/Input/IA_Jump.IA_Jump"))
  ;[1 1 1] 점프
  (:`Started`
    (`self.Jump`)))

(event `EnhancedInput|/Game/01_Blueprint/Global/Input/IA_MoveFoward`
  (params (ActionValue :type "Float (double-precision)") (ElapsedSeconds :type "Float (double-precision)") (TriggeredSeconds :type "Float (double-precision)") (InputAction :type "InputAction Object Reference" :default "/Game/01_Blueprint/Global/Input/IA_MoveFoward.IA_MoveFoward"))
  (bind (_returnvalue_roll _returnvalue_pitch _returnvalue_yaw) (`KismetMathLibrary.BreakRotator` (`self.GetControlRotation`)))
  ;[1 1 1] 앞으로
  (:`Triggered`
    (`self.AddMovementInput` (`KismetMathLibrary.GetForwardVector` (`KismetMathLibrary.MakeRotator` 0.0 0.0 _returnvalue_yaw)) ActionValue)
    (set `self.IsMove` true :!label _label))
  (:`Completed`
    (set `self.IsMove` false :!label _label_2)))

(event `Key|H`
  (params (Key :type "Key Structure"))
  ;[1 1 1] 디졸브
  (:`Pressed`
    (set `self.DissolveOn` (not (`self.DissolveOn`)))))

(event `self.ReceiveTick`
  (params (DeltaSeconds :type "Float (single-precision)"))
  (`|ExecutionSequence`
    (:`then_0`
      ;[1 1 1] 디졸브
      (`self.Dissolve` DeltaSeconds DeltaSeconds))))

(event `EnhancedInput|/Game/01_Blueprint/Global/Input/IA_MoveRight`
  (params (ActionValue :type "Float (double-precision)") (ElapsedSeconds :type "Float (double-precision)") (TriggeredSeconds :type "Float (double-precision)") (InputAction :type "InputAction Object Reference" :default "/Game/01_Blueprint/Global/Input/IA_MoveRight.IA_MoveRight"))
  (bind (_returnvalue_roll _returnvalue_pitch _returnvalue_yaw) (`KismetMathLibrary.BreakRotator` (`self.GetControlRotation`)))
  ;[1 1 1] 옆으로
  (:`Triggered`
    (`self.AddMovementInput` (`KismetMathLibrary.GetRightVector` (`KismetMathLibrary.MakeRotator` 0.0 0.0 _returnvalue_yaw)) ActionValue)
    (goto _label))
  (:`Completed`
    (goto _label_2)))

(event `EnhancedInput|/Game/01_Blueprint/Global/Input/IA_Light`
  (params (ActionValue :type Boolean) (ElapsedSeconds :type "Float (double-precision)") (TriggeredSeconds :type "Float (double-precision)") (InputAction :type "InputAction Object Reference" :default "/Game/01_Blueprint/Global/Input/IA_Light.IA_Light"))
  ;[1 1 1] 라이트
  (:`Started`
    (if (`self.IsLight`)
      (`LightComponent.SetIntensity` (`self.SpotLight`) 0.0)
      (set `self.IsLight` false)
      (else
        (`LightComponent.SetIntensity` (`self.SpotLight`) 10000.0)
        (set `self.IsLight` true)))))

(event `EnhancedInput|/Game/01_Blueprint/Global/Input/IA_MouseXY`
  (params (ActionValue :type "Vector2D Structure") (ElapsedSeconds :type "Float (double-precision)") (TriggeredSeconds :type "Float (double-precision)") (InputAction :type "InputAction Object Reference" :default "/Game/01_Blueprint/Global/Input/IA_MouseXY.IA_MouseXY"))
  ;[1 1 1] 마우스 회전
  (:`Triggered`
    (`self.AddControllerYawInput` ActionValue_X)
    (`self.AddControllerPitchInput` ActionValue_Y)))

(event `EnhancedInput|/Game/01_Blueprint/Global/Input/IA_Dance`
  (params (ActionValue :type Boolean) (ElapsedSeconds :type "Float (double-precision)") (TriggeredSeconds :type "Float (double-precision)") (InputAction :type "InputAction Object Reference" :default "/Game/01_Blueprint/Global/Input/IA_Dance.IA_Dance"))
  ;[1 1 1] 춤
  (:`Triggered`
    (`|PlayMontage` (`self.Mesh`) "/Game/02_Resource/Character/Skeleton/MixamoAni/Sk_Dance.Sk_Dance"
      (:`then`
        (set `self.IsDance` false)))))

(event `EnhancedInput|/Game/01_Blueprint/Global/Input/IA_MouseWheel`
  (params (ActionValue :type "Float (double-precision)") (ElapsedSeconds :type "Float (double-precision)") (TriggeredSeconds :type "Float (double-precision)") (InputAction :type "InputAction Object Reference" :default "/Game/01_Blueprint/Global/Input/IA_MouseWheel.IA_MouseWheel"))
  (bind _springarm (`self.SpringArm`))
  ;[1 1 1] 확대 축소
  (:`Triggered`
    (set `SpringArmComponent.TargetArmLength` (`KismetMathLibrary.FClamp` (+ (* ActionValue 10.0) (`SpringArmComponent.TargetArmLength` _springarm)) 100.0 1100.0) _springarm)))

(event `AttackCheck`
  (bind _returnvalue (`SceneComponent.K2_GetComponentLocation` (`self.Skeleton_Axe`)))
  ;[1 1 1] 공격 판정
  (bind (_outhit _returnvalue_2) (`KismetSystemLibrary.SphereTraceSingleByProfile` :`Start` _returnvalue :`End` (+ _returnvalue (* (`self.GetActorForwardVector`) 50.0)) :`Radius` 50.0 :`ProfileName` "PlayerAttack" :`DrawDebugType` "ForDuration"))
  (if _returnvalue_2
    (bind _returnvalue_3 (`NiagaraFunctionLibrary.SpawnSystemAtLocation` "/Game/02_Resource/Niagara/NA_AttackEffect.NA_AttackEffect" (`.Location` (`GameplayStatics.BreakHitResult` _outhit))))
    (`NiagaraComponent.SetNiagaraVariableFloat` _returnvalue_3 "MaxSize" 20.0)))

(event `EnhancedInput|/Game/01_Blueprint/Global/Input/IA_MouseLeftClick`
  (params (ActionValue :type Boolean) (ElapsedSeconds :type "Float (double-precision)") (TriggeredSeconds :type "Float (double-precision)") (InputAction :type "InputAction Object Reference" :default "/Game/01_Blueprint/Global/Input/IA_MouseLeftClick.IA_MouseLeftClick"))
  ;[1 1 1] 공격(마우스 우클릭)
  (:`Started`
    (if (`self.IsAttack`)
      (set `self.AttackSave` true)
      (else
        (switch `int` (`self.ComboCount`) :!label _label_3
          (:`0`
            (`|PlayMontage` (`self.Mesh`) "/Game/02_Resource/Character/Skeleton/BlendAnimation/AMT/AMT_Attack_Chop.AMT_Attack_Chop"
              (:`then`
                (set `self.IsAttack` true)
                (set `self.ComboCount` 1))))
          (:`1`
            (`|PlayMontage` (`self.Mesh`) "/Game/02_Resource/Character/Skeleton/BlendAnimation/AMT/AMT_Attack_Slice.AMT_Attack_Slice"
              (:`then`
                (set `self.IsAttack` true)
                (set `self.ComboCount` 2))))
          (:`2`
            (`|PlayMontage` (`self.Mesh`) "/Game/02_Resource/Character/Skeleton/BlendAnimation/AMT/AMT_Attack_Spin.AMT_Attack_Spin"
              (:`then`
                (set `self.IsAttack` true)
                (set `self.ComboCount` 3))))
          (:`3`
            (`|PlayMontage` (`self.Mesh`) "/Game/02_Resource/Character/Skeleton/BlendAnimation/AMT/AMT_Shoot.AMT_Shoot"
              (:`then`
                (set `self.IsAttack` true)
                (set `self.ComboCount` 0)))))))))

(event `ComboAction`
  ;[1 1 1] 공격(마우스 우클릭)
  (if (`self.AttackSave`)
    (set `self.AttackSave` false)
    (goto _label_3)))

(event `FootStep`
  (params (IsLeft :type Boolean))
  (`self.Func_FootStep` IsLeft))

(event `ResetCombo`
  ;[1 1 1] 공격(마우스 우클릭)
  (set `self.AttackSave` false)
  (set `self.ComboCount` 0)
  (set `self.IsAttack` false))

(fn `Dissolve`
  (params (B :type "Float (double-precision)") (B2 :type "Float (double-precision)"))
  (bind _dissolvetime (`self.Dissolvetime`))
  (bind _dissolvetime_2 (`self.Dissolvetime`))
  (bind _dissolvetime_3 (`self.Dissolvetime`))
  (if (`self.DissolveOn`)
    (if (> _dissolvetime -1.0)
      (bind _output_get (set `self.Dissolvetime` (- _dissolvetime B2)))
      (`MeshComponent.SetScalarParameterValueOnMaterials` (`self.Mesh`) "Dissolve" _output_get)
      (`MeshComponent.SetScalarParameterValueOnMaterials` (`self.Skeleton_Axe`) "Dissolve" _dissolvetime_3))
    (elif (< _dissolvetime_2 2.0)
      (bind _output_get_2 (set `self.Dissolvetime` (+ _dissolvetime_2 B)))
      (`MeshComponent.SetScalarParameterValueOnMaterials` (`self.Mesh`) "Dissolve" _output_get_2)
      (`MeshComponent.SetScalarParameterValueOnMaterials` (`self.Skeleton_Axe`) "Dissolve" _dissolvetime_3))))

(fn `Func_FootStep`
  (params (IsLeft :type Boolean))
  (bind _footlocation (`self.FootLocation`))
  (bind _returnvalue (`SceneComponent.K2_GetComponentRotation` (`self.Mesh`)))
  (if IsLeft
    (set `self.FootLocation` (`SceneComponent.GetSocketLocation` (`self.Mesh`) "toes_l"))
    (else
      (set `self.FootLocation` (`SceneComponent.GetSocketLocation` (`self.Mesh`) "toes_r"))))
  (bind (_outhit _returnvalue_2) (`KismetSystemLibrary.LineTraceSingle` :`Start` _footlocation :`End` (+ _footlocation (0.0 0.0 -20.0)) :`TraceChannel` "TraceTypeQuery3" :`DrawDebugType` "ForDuration" :`DrawTime` 2.0))
  (if _returnvalue_2
    (bind (_bblockinghit _binitialoverlap _time _distance _location _impactpoint _normal _impactnormal _physmat) (`GameplayStatics.BreakHitResult` _outhit))
    (bind _aspm_nd (cast `/Game/02_Resource/MTRL/PM_ND` _physmat)
      (:`then`
        (`NiagaraFunctionLibrary.SpawnSystemAtLocation` (`/Game/02_Resource/MTRL/PM_ND.NaFootWalk` _aspm_nd) _impactpoint _returnvalue)
        (`GameplayStatics.PlaySoundAtLocation` (`/Game/02_Resource/MTRL/PM_ND.FootSound` _aspm_nd) _impactpoint (struct) 1.0 1.0 0.0 null null null null)
        (`|SpawnActorFromClass` (`/Game/02_Resource/MTRL/PM_ND.FootPrint` _aspm_nd) (`KismetMathLibrary.MakeTransform` _impactpoint (`KismetMathLibrary.ComposeRotators` _returnvalue (struct :`Yaw` 90.0))) "Undefined" "MultiplyWithRoot" null null))
      (:`CastFailed`
        (`KismetSystemLibrary.PrintString` "Hello")))
    (else
      (`KismetSystemLibrary.PrintString` "NO"))))

(fn `Shooting`
  (bind (_returnvalue_location _returnvalue_rotation) (`KismetMathLibrary.BreakTransform` (`self.GetTransform`)))
  (`|SpawnActorFromClass` "/Game/01_Blueprint/Character/BP_ShootingBall.BP_ShootingBall_C" (`KismetMathLibrary.MakeTransform` (+ (* (`self.GetActorForwardVector`) 200.0) _returnvalue_location) _returnvalue_rotation) "Undefined" "MultiplyWithRoot" null null)
  (`NiagaraFunctionLibrary.SpawnSystemAtLocation` "/Game/02_Resource/Niagara/NA_FireEffect.NA_FireEffect" (+ (`SceneComponent.K2_GetComponentLocation` (`self.Skeleton_Axe`)) (* (`self.GetActorForwardVector`) 50.0))))

(fn `UserConstructionScript`)